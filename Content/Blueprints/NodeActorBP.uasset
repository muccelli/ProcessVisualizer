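; NodeActorBP is a labeled node actor that shows a configurable mesh and material, scaled by its significance.
; Its setup event creates a text render component offset by the mesh's bounds, then applies mesh, material and scale.
; Each tick turns the label toward the camera and swaps materials by camera distance, intended to make nearby nodes transparent.
; A MoveWidget function, not called here, raises a widget by mesh scale with a minimum height.
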(event Custom|SetNodeLabelAndTransform_1
  (bind _significancescale (Variables|Default|GetSignificanceScale))
  (bind _returnvalue (* _significancescale 1.5))
  (CallFunction|SetText)
  (Rendering|Material|SetMaterial (Variables|Default|GetVisualMesh) 0 (Variables|Default|GetNodeMeshMaterial))
  (Components|StaticMesh|SetStaticMesh (Variables|Default|GetVisualMesh) (Variables|Default|GetNodeMesh))
  (Transformation|SetWorldScale3D (Variables|Default|GetVisualMesh) (Math|Vector|MakeVector _returnvalue _returnvalue _returnvalue)))

(event EventTick
  (params (DeltaSeconds :type Float%20%28single-precision%29))
  (CallFunction|RotateText)
  ;[1 1 1] Try to make the nodes transparent when too close to the camera
  (Math|Float|CompareFloat (Math|Vector|Distance(Vector) (Transformation|GetActorLocation) (Camera|GetCameraLocation (Game|GetPlayerCameraManager 0))) 5e+02
    (:>
      (Rendering|Material|SetMaterial (Variables|Default|GetVisualMesh) 0 (Variables|Default|GetNodeMeshMaterial)))
    (:<
      (Rendering|Material|SetMaterial (Variables|Default|GetVisualMesh) 0 "/Game/Materials/M_StartEndNodesColor.M_StartEndNodesColor"))))

(fn ConstructionScript)

(fn RotateText
  (bind _labeltext_0 (Variables|Default|GetLabelText_0))
  (Transformation|SetWorldRotation _labeltext_0 (Math|Rotator|FindLookatRotation (Transformation|GetWorldLocation _labeltext_0) (Camera|GetCameraLocation (Game|GetPlayerCameraManager 0))) false false))

(fn MoveWidget
  (bind _widget (Variables|Default|GetWidget))
  (bind _visualmesh (Variables|Default|GetVisualMesh))
  (bind _relativescale3d (Variables|/Script/Engine.SceneComponent|GetRelativeScale3D _visualmesh))
  (bind _relativelocation (Variables|/Script/Engine.SceneComponent|GetRelativeLocation _widget))
  (bind _z (Math|Vector|BreakVector _relativelocation))
  (bind _z_2 (Math|Vector|BreakVector _relativescale3d))
  (bind _returnvalue (* _z_2 1e+02))
  (bind _returnvalue_2 (+ _z _returnvalue))
  (if (< _returnvalue_2 4e+01)
    (Transformation|SetRelativeLocation _widget (Math|Vector|MakeVector 0.0 0.0 4e+01) false false)
    (else
      (Transformation|SetRelativeLocation _widget (Math|Vector|MakeVector 0.0 0.0 _returnvalue_2) false false))))

(fn SetText
  (bind _visualmesh (Variables|Default|GetVisualMesh))
  (bind (_min _max) (Components|StaticMesh|GetLocalBounds _visualmesh))
  (bind _returnvalue (AddComponent|AddTextRenderComponent false (Math|Transform|MakeTransform (Math|Vector|MakeVector 0.0 0.0 (* (.z (Transformation|GetWorldScale _visualmesh)) (/ (- (.z _max) (.z _min)) 2.0))) (Math|Conversions|RotationFromXVector (* "0, 0, 0" -1.0)))))
  (bind _output_get (Variables|Default|SetLabelText_0 _returnvalue))
  (Rendering|Components|TextRender|SetText _output_get (Utilities|Text|ToText(String) (Variables|Default|GetLabel))))