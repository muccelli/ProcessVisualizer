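; Directed graph edge actor, drawn as spline meshes with an arrowhead pointing at its ToNode.
; SetEdgeProperties builds a flattened segment per spline span, shortening the last to clear the node's radius and arrowhead, then caches the point data.
; SignificanceScale drives thickness, TimeScale feeds the dynamic material's ColorAlpha, and SetNewMaterial toggles highlighting.
; Percentage label and mesh-update helpers exist, but their calls within the event graph are disconnected.
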(event EventTick
  (params (DeltaSeconds :type Float%20%28single-precision%29)))

(event EventSetEdgeProperties
  (Utilities|FlowControl|Sequence
    (:then_0
      (Variables|Default|SetNumberOfSplinePoints (Spline|GetNumberOfSplinePoints (Variables|Default|GetSpline))))
    (:then_1
      (Utilities|FlowControl|Sequence
        (:then_0
          (for _index (range 0 (- (Variables|Default|GetNumberOfSplinePoints) 2))
            (CallFunction|BuildEdgeElement _index (Variables|Default|GetEdgeMesh))))
        (:then_1
          (for _index_2 (range 0 (- (Variables|Default|GetNumberOfSplinePoints) 1))
            (Utilities|Array|Add (Variables|Default|GetSplineDataArray) (Utilities|Struct|MakeSplinePointData (.Location (Spline|GetLocationandTangentatSplinePoint (Variables|Default|GetSpline) _index_2 "Local")) (.Tangent (Spline|GetLocationandTangentatSplinePoint (Variables|Default|GetSpline) _index_2 "Local"))))))))
    (:then_2)))

(fn ConstructionScript)

(fn BuildEdgeElement
  (params (LoopIndex :type Integer) (EdgeElementMesh :type Static%20Mesh%20Object%20Reference))
  (bind _spline (Variables|Default|GetSpline))
  (bind _significancescale (Variables|Default|GetSignificanceScale))
  (bind _numberofsplinepoints (Variables|Default|GetNumberOfSplinePoints))
  (bind _tonode (Variables|Default|GetToNode))
  (bind _significancescale_2 (Variables|Default|GetSignificanceScale))
  (bind _returnvalue (Actor|GetComponentbyClass _tonode "/Script/Engine.StaticMeshComponent"))
  (bind _returnvalue_2 (- _numberofsplinepoints 1))
  (bind _returnvalue_3 (* _significancescale_2 2.0))
  (bind (_min _max) (Components|StaticMesh|GetLocalBounds _returnvalue))
  (bind _tangent (Spline|GetLocationandTangentatSplinePoint _spline _returnvalue_2 "Local"))
  (bind _returnvalue_4 (Math|Conversions|RotationFromXVector _tangent))
  (bind (_roll _pitch _yaw) (Math|Rotator|BreakRotator _returnvalue_4))
  (LocalVariables|SetLocal_CurrentLoopIndex LoopIndex)
  (LocalVariables|SetLocal_NextLoopIndex (Math|Integer|%(Integer) (+ LoopIndex 1) (Variables|Default|GetNumberOfSplinePoints)))
  (LocalVariables|SetLocal_EdgeElementMesh EdgeElementMesh)
  (Utilities|FlowControl|Sequence
    (:then_0
      (LocalVariables|SetLocal_StartLocation (Math|Vector|MakeVector (.x (.Location (Spline|GetLocationandTangentatSplinePoint (Variables|Default|GetSpline) (LocalVariables|GetLocal_CurrentLoopIndex) "Local"))) (.y (.Location (Spline|GetLocationandTangentatSplinePoint (Variables|Default|GetSpline) (LocalVariables|GetLocal_CurrentLoopIndex) "Local"))) 5.0))
      (LocalVariables|SetLocal_StartTangent (.Tangent (Spline|GetLocationandTangentatSplinePoint (Variables|Default|GetSpline) (LocalVariables|GetLocal_CurrentLoopIndex) "Local")))
      (LocalVariables|SetLocal_EndLocation (Math|Vector|MakeVector (.x (select (== (LocalVariables|GetLocal_NextLoopIndex) (- (Variables|Default|GetNumberOfSplinePoints) 1)) (- (LocalVariables|GetLocal_StartLocation) (* (Math|Vector|Normalize (- (LocalVariables|GetLocal_StartLocation) (.Location (Spline|GetLocationandTangentatSplinePoint (Variables|Default|GetSpline) (- (Variables|Default|GetNumberOfSplinePoints) 1) "Local")))) (- (Math|Vector|VectorLength (- (LocalVariables|GetLocal_StartLocation) (.Location (Spline|GetLocationandTangentatSplinePoint (Variables|Default|GetSpline) (- (Variables|Default|GetNumberOfSplinePoints) 1) "Local")))) (+ (* (.x (Transformation|GetWorldScale _returnvalue)) (/ (- (.x _max) (.x _min)) 2.0)) (* (Variables|Default|GetSignificanceScale) 99.0))))) (.Location (Spline|GetLocationandTangentatSplinePoint (Variables|Default|GetSpline) (LocalVariables|GetLocal_NextLoopIndex) "Local")))) (.y (select (== (LocalVariables|GetLocal_NextLoopIndex) (- (Variables|Default|GetNumberOfSplinePoints) 1)) (- (LocalVariables|GetLocal_StartLocation) (* (Math|Vector|Normalize (- (LocalVariables|GetLocal_StartLocation) (.Location (Spline|GetLocationandTangentatSplinePoint (Variables|Default|GetSpline) (- (Variables|Default|GetNumberOfSplinePoints) 1) "Local")))) (- (Math|Vector|VectorLength (- (LocalVariables|GetLocal_StartLocation) (.Location (Spline|GetLocationandTangentatSplinePoint (Variables|Default|GetSpline) (- (Variables|Default|GetNumberOfSplinePoints) 1) "Local")))) (+ (* (.x (Transformation|GetWorldScale _returnvalue)) (/ (- (.x _max) (.x _min)) 2.0)) (* (Variables|Default|GetSignificanceScale) 99.0))))) (.Location (Spline|GetLocationandTangentatSplinePoint (Variables|Default|GetSpline) (LocalVariables|GetLocal_NextLoopIndex) "Local")))) 5.0))
      (LocalVariables|SetLocal_EndTangent (.Tangent (Spline|GetLocationandTangentatSplinePoint (Variables|Default|GetSpline) (LocalVariables|GetLocal_NextLoopIndex) "Local")))
      (LocalVariables|SetLocal_StartScale (Math|Vector2D|MakeVector2D _returnvalue_3 0.001))
      (LocalVariables|SetLocal_EndScale (Math|Vector2D|MakeVector2D _returnvalue_3 0.001)))
    (:then_1
      (bind _returnvalue_5 (AddComponent|AddSplineMeshComponent false))
      (Utilities|Array|Add (Variables|Default|GetSplineMeshComponents) _returnvalue_5)
      (LocalVariables|SetLocal_CurrentSplineMesh _returnvalue_5)
      (SplineMesh|SetForwardAxis (LocalVariables|GetLocal_CurrentSplineMesh) "Z" true)
      (Components|StaticMesh|SetStaticMesh (LocalVariables|GetLocal_CurrentSplineMesh) (LocalVariables|GetLocal_EdgeElementMesh))
      (SplineMesh|SetStartandEnd (LocalVariables|GetLocal_CurrentSplineMesh) (LocalVariables|GetLocal_StartLocation) (LocalVariables|GetLocal_StartTangent) (LocalVariables|GetLocal_EndLocation) (LocalVariables|GetLocal_EndTangent) true :!class /Script/Engine.SplineMeshComponent)
      (SplineMesh|SetStartScale (LocalVariables|GetLocal_CurrentSplineMesh) (LocalVariables|GetLocal_StartScale) true :!class /Script/Engine.SplineMeshComponent)
      (SplineMesh|SetEndScale (LocalVariables|GetLocal_CurrentSplineMesh) (LocalVariables|GetLocal_EndScale) true :!class /Script/Engine.SplineMeshComponent)
      (bind _returnvalue_6 (Rendering|Material|CreateDynamicMaterialInstance (LocalVariables|GetLocal_CurrentSplineMesh) 0 (Variables|Default|GetEdgeMeshMaterial) "None" :!class /Script/Engine.PrimitiveComponent))
      (bind _output_get (Variables|Default|SetDynamicEdgeMaterial _returnvalue_6))
      (Rendering|Material|SetScalarParameterValue _output_get "ColorAlpha" (Variables|Default|GetTimeScale) :!class /Script/Engine.MaterialInstanceDynamic))
    (:then_2
      (if (== (LocalVariables|GetLocal_NextLoopIndex) (- (Variables|Default|GetNumberOfSplinePoints) 1))
        (bind _returnvalue_7 (AddComponent|AddStaticMeshComponent false (Math|Transform|MakeTransform (LocalVariables|GetLocal_EndLocation) (Math|Rotator|MakeRotator _roll (+ _pitch -9e+01) _yaw))))
        (Variables|Default|SetArrowMesh _returnvalue_7)
        (Components|StaticMesh|SetStaticMesh _returnvalue_7 (Variables|Default|GetEdgeHeadMesh))
        (Rendering|Material|SetMaterial _returnvalue_7 0 (Variables|Default|GetDynamicEdgeMaterial))
        (Transformation|SetWorldScale3D _returnvalue_7 (* (Math|Vector|MakeVector 0.001 (* _significancescale 2.0) _significancescale) 2.0))))))

(fn CreateText
  (bind _spline (Variables|Default|GetSpline))
  (bind (_location _tangent) (Spline|GetLocationandTangentatSplinePoint _spline 1 "Local"))
  (bind (_x _y _z) (Math|Vector|BreakVector _location))
  (bind _returnvalue (AddComponent|AddTextRenderComponent false (Math|Transform|MakeTransform (Math|Vector|MakeVector (+ _x 0.0) _y (+ _z 1e+01)) (Math|Conversions|RotationFromXVector (* _tangent -1.0)))))
  (bind _output_get (Variables|Default|SetSignificanceText _returnvalue))
  (CallFunction|SetText _output_get))

(fn UpdateSplineMeshesLocation
  (bind _spline (Variables|Default|GetSpline))
  (bind _significancescale (Variables|Default|GetSignificanceScale))
  (bind _numberofsplinepoints (Variables|Default|GetNumberOfSplinePoints))
  (bind _returnvalue (- _numberofsplinepoints 1))
  (bind _tangent (Spline|GetLocationandTangentatSplinePoint _spline _returnvalue "Local"))
  (bind _returnvalue_2 (Math|Conversions|RotationFromXVector _tangent))
  (bind (_roll _pitch _yaw) (Math|Rotator|BreakRotator _returnvalue_2))
  (for _index (range 0 (- (Variables|Default|GetNumberOfSplinePoints) 2))
    (bind _output_get (LocalVariables|SetLocal_CurrentLoopIndex _index))
    (LocalVariables|SetLocal_NextLoopIndex (Math|Integer|%(Integer) (+ _index 1) (Variables|Default|GetNumberOfSplinePoints)))
    (SplineMesh|SetStartandEnd (Utilities|Array|Get(acopy) (Variables|Default|GetSplineMeshComponents) _output_get) (.Location (Spline|GetLocationandTangentatSplinePoint (Variables|Default|GetSpline) (LocalVariables|GetLocal_CurrentLoopIndex) "Local")) (.Tangent (Spline|GetLocationandTangentatSplinePoint (Variables|Default|GetSpline) (LocalVariables|GetLocal_CurrentLoopIndex) "Local")) (select (== (LocalVariables|GetLocal_NextLoopIndex) (- (Variables|Default|GetNumberOfSplinePoints) 1)) (|ShortenForArrow) (.Location (Spline|GetLocationandTangentatSplinePoint (Variables|Default|GetSpline) (LocalVariables|GetLocal_NextLoopIndex) "Local"))) (.Tangent (Spline|GetLocationandTangentatSplinePoint (Variables|Default|GetSpline) (LocalVariables|GetLocal_NextLoopIndex) "Local")) true :!class /Script/Engine.SplineMeshComponent))
  (Transformation|SetWorldTransform (Variables|Default|GetArrowMesh) (Math|Transform|MakeTransform (|ShortenForArrow_2) (Math|Rotator|MakeRotator _roll (+ _pitch -9e+01) _yaw) (* (Math|Vector|MakeVector 0.0 (* _significancescale 2.0) _significancescale) 2.0)) false false))

(fn SetText
  (params (self2 :type Text%20Render%20Component%20Object%20Reference))
  (Rendering|Components|TextRender|SetText self2 (Utilities|Text|ToText(String) (Utilities|String|BuildString(Float) "" "" (/ (Math|Conversions|ToFloat(Integer) (Math|Float|Round (* (Variables|Default|GetPercentageFrequencyToTotal) 1e+02))) 1e+02) "%"))))

(fn SetNewMaterial
  (params (ToHighlight :type Boolean))
  (LocalVariables|SetLocal_NewMaterial "/Game/Materials/M_EdgesColorHighlight.M_EdgesColorHighlight")
  (if ToHighlight
    (for _array_element (Variables|Default|GetSplineMeshComponents)
      (Rendering|Material|SetMaterial _array_element 0 (LocalVariables|GetLocal_NewMaterial)))
    (Rendering|Material|SetMaterial (Variables|Default|GetArrowMesh) 0 (LocalVariables|GetLocal_NewMaterial))
    (else
      (for _array_element_2 (Variables|Default|GetSplineMeshComponents)
        (bind _returnvalue (Rendering|Material|CreateDynamicMaterialInstance _array_element_2 0 (Variables|Default|GetEdgeMeshMaterial) "None" :!class /Script/Engine.PrimitiveComponent))
        (bind _output_get (Variables|Default|SetDynamicEdgeMaterial _returnvalue))
        (Rendering|Material|SetScalarParameterValue _output_get "ColorAlpha" (Variables|Default|GetTimeScale) :!class /Script/Engine.MaterialInstanceDynamic))
      (Rendering|Material|SetMaterial (Variables|Default|GetArrowMesh) 0 (Variables|Default|GetDynamicEdgeMaterial)))))