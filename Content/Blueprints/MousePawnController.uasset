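; MousePawnController is a mouse-driven camera pawn with height, yaw and zoom control.
; Mouse Y sets actor height through a scaled, inverted offset, leaving the location's X and Y inputs at zero.
; Mouse X adds yaw input, then resets the first player controller's pitch and roll to zero.
; The mouse wheel changes spring arm length in fixed, unclamped steps.
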(event Input|MouseEvents|MouseX
  (params (AxisValue :type Float%20%28single-precision%29))
  (bind _returnvalue (Game|GetPlayerController 0))
  (Pawn|Input|AddControllerYawInput AxisValue)
  (Pawn|SetControlRotation _returnvalue (Math|Rotator|MakeRotator 0.0 0.0 (.yaw (Pawn|GetControlRotation _returnvalue :!class /Script/Engine.Controller)))))

(event Input|MouseEvents|MouseY
  (params (AxisValue :type Float%20%28single-precision%29))
  (Transformation|SetActorLocation (Math|Vector|MakeVector 0.0 0.0 (.z (+ (Math|Vector|MakeVector 0.0 0.0 (.z (Transformation|GetActorLocation))) (* AxisValue -1e+02)))) false false))

(event Input|MouseEvents|MouseWheelUp
  (params (Key :type Key%20Structure :default "None"))
  (bind _springarm (Variables|Default|GetSpringArm))
  (:Pressed
    (Variables|/Script/Engine.SpringArmComponent|SetTargetArmLength _springarm (+ (Variables|/Script/Engine.SpringArmComponent|GetTargetArmLength _springarm) -2e+02))))

(event Input|MouseEvents|MouseWheelDown
  (params (Key :type Key%20Structure :default "None"))
  (bind _springarm (Variables|Default|GetSpringArm))
  (:Pressed
    (Variables|/Script/Engine.SpringArmComponent|SetTargetArmLength _springarm (+ (Variables|/Script/Engine.SpringArmComponent|GetTargetArmLength _springarm) 2e+02))))

(fn ConstructionScript)