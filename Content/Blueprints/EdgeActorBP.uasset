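; Directed graph edge actor that draws a weighted arrow along a spline toward ToNode, labelled with its Significance.
; SetEdgeProperties builds Significance-scaled spline meshes, shortens the last for an arrowhead outside the node's sphere, caches point data and adds the text.
; Tick turns the label toward the camera and compares spline points against the cache to reposition segments on change.
; These updates neither move the arrowhead nor reapply the shortening.
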(event EventTick
  (params (DeltaSeconds :type Float%20%28single-precision%29))
  (bind _significancetext (Variables|Default|GetSignificanceText))
  (Transformation|SetWorldRotation _significancetext (Math|Rotator|FindLookatRotation (Transformation|GetWorldLocation _significancetext) (Camera|GetCameraLocation (Game|GetPlayerCameraManager 0))) false false)
  (for _index (range 0 (- (Variables|Default|GetNumberOfSplinePoints) 1))
    (if (or (Math|Vector|NotEqual(Vector) (.location (Utilities|Array|Get(acopy) (Variables|Default|GetSplineDataArray) _index)) (.Location (Spline|GetLocationandTangentatSplinePoint (Variables|Default|GetSpline) _index "Local")) 0.0001) (Math|Vector|NotEqual(Vector) (.tangent (Utilities|Array|Get(acopy) (Variables|Default|GetSplineDataArray) _index)) (.Tangent (Spline|GetLocationandTangentatSplinePoint (Variables|Default|GetSpline) _index "Local")) 0.0001))
      (CallFunction|UpdateSplineMeshesLocation)
      (for _index_2 (range 0 (- (Variables|Default|GetNumberOfSplinePoints) 1))
        (Utilities|Array|SetArrayElem (Variables|Default|GetSplineDataArray) 0 (Utilities|Struct|MakeSplinePointData (.Location (Spline|GetLocationandTangentatSplinePoint (Variables|Default|GetSpline) _index_2 "Local")) (.Tangent (Spline|GetLocationandTangentatSplinePoint (Variables|Default|GetSpline) _index_2 "Local"))))))))

(event EventSetEdgeProperties
  (Utilities|FlowControl|Sequence
    (:then_0
      (Variables|Default|SetNumberOfSplinePoints (Spline|GetNumberOfSplinePoints (Variables|Default|GetSpline))))
    (:then_1
      (Utilities|FlowControl|Sequence
        (:then_0
          (for _index (range 0 (- (Variables|Default|GetNumberOfSplinePoints) 2))
            (CallFunction|BuildEdgeElement _index (Variables|Default|GetEdgeMesh))))
        (:then_1
          (for _index_2 (range 0 (- (Variables|Default|GetNumberOfSplinePoints) 1))
            (Utilities|Array|Add (Variables|Default|GetSplineDataArray) (Utilities|Struct|MakeSplinePointData (.Location (Spline|GetLocationandTangentatSplinePoint (Variables|Default|GetSpline) _index_2 "Local")) (.Tangent (Spline|GetLocationandTangentatSplinePoint (Variables|Default|GetSpline) _index_2 "Local"))))))))
    (:then_2
      (CallFunction|SetSignificanceText))
    (:then_3)))

(fn ConstructionScript)

(fn BuildEdgeElement
  (params (LoopIndex :type Integer) (EdgeElementMesh :type Static%20Mesh%20Object%20Reference))
  (bind _spline (Variables|Default|GetSpline))
  (bind _significance (Variables|Default|GetSignificance))
  (bind _numberofsplinepoints (Variables|Default|GetNumberOfSplinePoints))
  (bind _significance_2 (Variables|Default|GetSignificance))
  (bind _tonode (Variables|Default|GetToNode))
  (bind _returnvalue (- _numberofsplinepoints 1))
  (bind _spherevisual (Variables|/Script/ProcessVisualizer.NodeActor|GetSphereVisual _tonode))
  (bind (_min _max) (Components|StaticMesh|GetLocalBounds _spherevisual))
  (bind _tangent (Spline|GetLocationandTangentatSplinePoint _spline _returnvalue "Local"))
  (bind _returnvalue_2 (Math|Conversions|RotationFromXVector _tangent))
  (bind (_roll _pitch _yaw) (Math|Rotator|BreakRotator _returnvalue_2))
  (LocalVariables|SetLocal_CurrentLoopIndex LoopIndex)
  (LocalVariables|SetLocal_NextLoopIndex (Math|Integer|%(Integer) (+ LoopIndex 1) (Variables|Default|GetNumberOfSplinePoints)))
  (LocalVariables|SetLocal_EdgeElementMesh EdgeElementMesh)
  (Utilities|FlowControl|Sequence
    (:then_0
      (LocalVariables|SetLocal_StartLocation (.Location (Spline|GetLocationandTangentatSplinePoint (Variables|Default|GetSpline) (LocalVariables|GetLocal_CurrentLoopIndex) "Local")))
      (LocalVariables|SetLocal_StartTangent (.Tangent (Spline|GetLocationandTangentatSplinePoint (Variables|Default|GetSpline) (LocalVariables|GetLocal_CurrentLoopIndex) "Local")))
      (LocalVariables|SetLocal_EndLocation (select (== (LocalVariables|GetLocal_NextLoopIndex) (- (Variables|Default|GetNumberOfSplinePoints) 1)) (- (LocalVariables|GetLocal_StartLocation) (* (Math|Vector|Normalize (- (LocalVariables|GetLocal_StartLocation) (.Location (Spline|GetLocationandTangentatSplinePoint (Variables|Default|GetSpline) (- (Variables|Default|GetNumberOfSplinePoints) 1) "Local")))) (- (Math|Vector|VectorLength (- (LocalVariables|GetLocal_StartLocation) (.Location (Spline|GetLocationandTangentatSplinePoint (Variables|Default|GetSpline) (- (Variables|Default|GetNumberOfSplinePoints) 1) "Local")))) (+ (* (.x (Transformation|GetWorldScale _spherevisual)) (/ (- (.x _max) (.x _min)) 2.0)) (* (Variables|Default|GetSignificance) 99.0))))) (.Location (Spline|GetLocationandTangentatSplinePoint (Variables|Default|GetSpline) (LocalVariables|GetLocal_NextLoopIndex) "Local"))))
      (LocalVariables|SetLocal_EndTangent (.Tangent (Spline|GetLocationandTangentatSplinePoint (Variables|Default|GetSpline) (LocalVariables|GetLocal_NextLoopIndex) "Local")))
      (LocalVariables|SetLocal_StartScale (Math|Vector2D|MakeVector2D _significance_2 _significance_2))
      (LocalVariables|SetLocal_EndScale (Math|Vector2D|MakeVector2D _significance_2 _significance_2)))
    (:then_1
      (bind _returnvalue_3 (AddComponent|AddSplineMeshComponent false))
      (Utilities|Array|Add (Variables|Default|GetSplineMeshComponents) _returnvalue_3)
      (LocalVariables|SetLocal_CurrentSplineMesh _returnvalue_3)
      (SplineMesh|SetForwardAxis (LocalVariables|GetLocal_CurrentSplineMesh) "Z" true)
      (Components|StaticMesh|SetStaticMesh (LocalVariables|GetLocal_CurrentSplineMesh) (LocalVariables|GetLocal_EdgeElementMesh))
      (SplineMesh|SetStartandEnd (LocalVariables|GetLocal_CurrentSplineMesh) (LocalVariables|GetLocal_StartLocation) (LocalVariables|GetLocal_StartTangent) (LocalVariables|GetLocal_EndLocation) (LocalVariables|GetLocal_EndTangent) true :!class /Script/Engine.SplineMeshComponent)
      (SplineMesh|SetStartScale (LocalVariables|GetLocal_CurrentSplineMesh) (LocalVariables|GetLocal_StartScale) true :!class /Script/Engine.SplineMeshComponent)
      (SplineMesh|SetEndScale (LocalVariables|GetLocal_CurrentSplineMesh) (LocalVariables|GetLocal_EndScale) true :!class /Script/Engine.SplineMeshComponent)
      (Rendering|Material|SetMaterial (LocalVariables|GetLocal_CurrentSplineMesh) 0 (Variables|Default|GetEdgeMeshMaterial))
      (Collision|SetCollisionEnabled (LocalVariables|GetLocal_CurrentSplineMesh) "QueryAndPhysics")
      (if (== (LocalVariables|GetLocal_NextLoopIndex) (- (Variables|Default|GetNumberOfSplinePoints) 1))
        (bind _returnvalue_4 (AddComponent|AddStaticMeshComponent false (Math|Transform|MakeTransform (LocalVariables|GetLocal_EndLocation) (Math|Rotator|MakeRotator _roll (+ _pitch -9e+01) _yaw))))
        (Components|StaticMesh|SetStaticMesh _returnvalue_4 (Variables|Default|GetEdgeHeadMesh))
        (Rendering|Material|SetMaterial _returnvalue_4 0 (Variables|Default|GetEdgeMeshMaterial))
        (Transformation|SetWorldScale3D _returnvalue_4 (* (Math|Vector|MakeVector _significance _significance _significance) 2.0))))))

(fn SetSignificanceText
  (bind _spline (Variables|Default|GetSpline))
  (bind (_location _tangent) (Spline|GetLocationandTangentatSplinePoint _spline 1 "Local"))
  (bind (_x _y _z) (Math|Vector|BreakVector _location))
  (bind _returnvalue (AddComponent|AddTextRenderComponent false (Math|Transform|MakeTransform (Math|Vector|MakeVector (+ _x 5e+01) _y (+ _z 5e+01)) (Math|Conversions|RotationFromXVector (* _tangent -1.0)))))
  (bind _output_get (Variables|Default|SetSignificanceText _returnvalue))
  (Rendering|Components|TextRender|SetText _output_get (Utilities|Text|ToText(Float) (Variables|Default|GetSignificance) "HalfToEven")))

(fn UpdateSplineMeshesLocation
  (for _index (range 0 (- (Variables|Default|GetNumberOfSplinePoints) 2))
    (LocalVariables|SetLocal_CurrentLoopIndex _index)
    (LocalVariables|SetLocal_NextLoopIndex (Math|Integer|%(Integer) (+ _index 1) (Variables|Default|GetNumberOfSplinePoints)))
    (LocalVariables|SetLocal_SplineMeshComponent (Utilities|Array|Get(acopy) (Variables|Default|GetSplineMeshComponents) (LocalVariables|GetLocal_CurrentLoopIndex)))
    (SplineMesh|SetStartandEnd (LocalVariables|GetLocal_SplineMeshComponent) (.Location (Spline|GetLocationandTangentatSplinePoint (Variables|Default|GetSpline) (LocalVariables|GetLocal_CurrentLoopIndex) "Local")) (.Tangent (Spline|GetLocationandTangentatSplinePoint (Variables|Default|GetSpline) (LocalVariables|GetLocal_CurrentLoopIndex) "Local")) (.Location (Spline|GetLocationandTangentatSplinePoint (Variables|Default|GetSpline) (LocalVariables|GetLocal_NextLoopIndex) "Local")) (.Tangent (Spline|GetLocationandTangentatSplinePoint (Variables|Default|GetSpline) (LocalVariables|GetLocal_NextLoopIndex) "Local")) true :!class /Script/Engine.SplineMeshComponent)))